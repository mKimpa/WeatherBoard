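; Weather board actor that shows temperature maps on a plane, either for a requested date-hour or as a looping playback.
; Date lookups in TemperatureData fall back to a default texture; the chosen map feeds a new dynamic material instance's TemperatureMask parameter.
; A one-second timer steps a counter through the data, wrapping before the last entry.
; Playback also splits each date string to update the control widget's date fields and hour slider.
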(event `self.ReceiveBeginPlay`)

(fn `DisplayData`
  (params (DataMap :type "Texture Object Reference"))
  (bind _returnvalue (`PrimitiveComponent.CreateDynamicMaterialInstance` (`self.Plane`) 0 "/Game/Textures+Materials/BaseMaterial.BaseMaterial" "None"))
  (`MaterialInstanceDynamic.SetTextureParameterValue` _returnvalue "TemperatureMask" DataMap))

(fn `GetDataMap`
  (params (`YYYY-MM-DD-HH` :type String))
  (returns (Texture :type "TextureParameterValue Structure"))
  (for _array_element (`self.TemperatureData`)
    (if (`KismetStringLibrary.EqualEqual_StrStr` (`.Date_8_9B3935624FDEFA53F67277B99919104F` (break `/Game/TempData` _array_element)) `YYYY-MM-DD-HH`)
      (return (break `/Game/TempData` _array_element))))
  (return (make `TextureParameterValue` (struct :`Association` "GlobalParameter" :`Index` -1) "/Engine/EngineMaterials/DefaultDiffuse_TC_Masks.DefaultDiffuse_TC_Masks")))

(fn `GetNextDataMap`
  (returns (DataMap :type "Texture Object Reference") (`YYYY-MM-DD-HH` :type String))
  (bind _temperaturedata (`self.TemperatureData`))
  (bind _output (`|GetArrayItem` _temperaturedata (mod (`self.Counter`) (- (`KismetArrayLibrary.Array_Length` _temperaturedata) 1))))
  (return (`.ParameterValue` (break `TextureParameterValue` (break `/Game/TempData` _output))) (`.Date_8_9B3935624FDEFA53F67277B99919104F` (break `/Game/TempData` _output))))

(fn `GetWiget`
  (returns (Wiget :type "/Game/Wigets/WeatherBoardControlWiget Object Reference"))
  (bind _foundwidgets (`WidgetBlueprintLibrary.GetAllWidgetsOfClass` "/Game/Wigets/WeatherBoardControlWiget.WeatherBoardControlWiget_C"))
  (return (`|GetArrayItem` _foundwidgets)))

(fn `LoadDataMap`
  (params (`YYYY-MM-DD-HH` :type String))
  (bind _texture (`self.GetDataMap` `YYYY-MM-DD-HH`))
  (`self.DisplayData` (`.ParameterValue` (break `TextureParameterValue` _texture))))

(fn `LoopData`
  (locals (NewLocalVar_0 :type "/Game/Wigets/WeatherBoardControlWiget Object Reference"))
  (bind (_datamap _yyyy_mm_dd_hh) (`self.GetNextDataMap`))
  (`self.DisplayData` _datamap)
  (`self.UpdateWigetControls` _yyyy_mm_dd_hh)
  (`/Engine/EditorBlueprintResources/StandardMacros.IncrementInt` (`self.Counter`)))

(fn `StartLoopingData`
  (bind _returnvalue (`KismetSystemLibrary.K2_SetTimer` null "LoopData" 1.0 true))
  (set `self.DataLoopHandler` _returnvalue))

(fn `StopLoopingData`
  (`KismetSystemLibrary.K2_ClearAndInvalidateTimerHandle` (`self.DataLoopHandler`)))

(fn `UpdateWigetControls`
  (params (SourceString :type String))
  (bind _returnvalue (`KismetStringLibrary.ParseIntoArray` SourceString "-"))
  (bind _output (`|GetArrayItem` _returnvalue 3))
  (bind _wiget (`self.GetWiget`))
  (`EditableTextBox.SetText` (`/Game/Wigets/WeatherBoardControlWiget.Year` _wiget) (`KismetTextLibrary.Conv_StringToText` (`|GetArrayItem` _returnvalue)))
  (`EditableTextBox.SetText` (`/Game/Wigets/WeatherBoardControlWiget.Month` _wiget) (`KismetTextLibrary.Conv_StringToText` (`|GetArrayItem` _returnvalue 1)))
  (`EditableTextBox.SetText` (`/Game/Wigets/WeatherBoardControlWiget.Day` _wiget) (`KismetTextLibrary.Conv_StringToText` (`|GetArrayItem` _returnvalue 2)))
  (`EditableTextBox.SetText` (`/Game/Wigets/WeatherBoardControlWiget.Hour` _wiget) (`KismetTextLibrary.Conv_StringToText` _output))
  (`Slider.SetValue` (`/Game/Wigets/WeatherBoardControlWiget.HourSlider` _wiget) (`KismetStringLibrary.Conv_StringToDouble` _output)))

(fn `UserConstructionScript`)